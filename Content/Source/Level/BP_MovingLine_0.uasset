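; Moving line level actor whose graphs only provide a debug preview of its layout in the construction script.
; When Debug is set, it adds a child actor of MovingSegmentClass and billboard markers at the left and right line spawn locations and the character stand location.
; The event graph holds only disabled placeholder events, so no movement or spawning logic runs in these graphs.
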(event EventBeginPlay)

(event Collision|EventActorBeginOverlap
  (params (OtherActor :type Actor%20Object%20Reference)))

(event EventTick
  (params (DeltaSeconds :type Float%20%28single-precision%29)))

(fn ConstructionScript
  (if (Variables|Default|GetDebug)
    (Utilities|FlowControl|Sequence
      (:then_0
        (bind _returnvalue (AddComponent|AddChildActorComponent true))
        (ChildActorComponent|SetChildActorClass _returnvalue (Variables|Default|GetMovingSegmentClass)))
      (:then_1
        (AddComponent|AddBillboardComponent true (Math|Transform|MakeTransform (Variables|Default|GetLeftLineSpawnLocation_) "0, 0, 0" "1,1,1"))
        (AddComponent|AddBillboardComponent true (Math|Transform|MakeTransform (Variables|Default|GetRightLineSpawnLocation_) "0, 0, 0" "1,1,1"))
        (AddComponent|AddBillboardComponent true (Math|Transform|MakeTransform (Variables|Default|GetCharacterStandLocation_) "0, 0, 0" "1,1,1"))))))