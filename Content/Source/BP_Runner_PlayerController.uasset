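; Player controller for a runner game that turns input actions and touch swipes into lane changes and up/down moves on the runner pawn.
; Swipes over a length threshold resolve by dominant axis into the same move events.
; Left/right ask the moving level for a line and send the pawn to its stand location, unless mid-vertical move.
; A control type enum gates movement, toggling input and cursor between Runner and Interface modes.
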(event Custom|PawnMoveTo
  (params (MovingLine :type Moving%20Line%20Object%20Reference))
  ;[0 0 0] Pawn Move To
  (Utilities|IsValid MovingLine
    (:Is%20Valid
      (bind _returnvalue (Class|MovingLine|GetCharacterStandLocation MovingLine))
      (Utilities|IsValid (Variables|Default|GetBP_RunnerPlayerPawn)
        (:Is%20Valid
          _)
        (:Is%20Not%20Valid
          (CallFunction|SavePawnRef)))
      (Default|Moveto (Variables|Default|GetBP_RunnerPlayerPawn) _returnvalue))))

(event Custom|PlayerDeath
  (CallFunction|SetControllType "NewEnumerator0"))

(event Custom|MoveUp
  ;[0 0 0] Moving Up
  (switch Utilities|FlowControl|Switch|SwitchonEControllType (Variables|Default|GetControllType)
    (:NewEnumerator1
      (Default|MovingUp (Variables|Default|GetBP_RunnerPlayerPawn)))))

(event Custom|Binds
  (bind _asbp_runner_player_pawn (Utilities|Casting|CastToBP_Runner_PlayerPawn (Game|Player|GetPlayerPawn 0)))
  (EventDispatchers|BindEventtoDeathDispatcher _asbp_runner_player_pawn (EventDispatchers|CreateEvent :!event Custom|PlayerDeath)))

(event Custom|CheckSwipe
  (bind (_locationx _locationy) (Class|PlayerController|GetInputTouchState "Touch1"))
  ;[0 0 0] Mobile Controlls
  (if (> (Math|Vector2D|Vector2DLength (- (Variables|Default|GetTouchStartLocation) (Variables|Default|GetTouchEndLocation))) 1e+02)
    (bind _output_get (Variables|Default|SetTouchEndLocation (Math|Vector2D|MakeVector2D _locationx _locationy)))
    (if (> (Math|Float|Absolute(Float) (.x (- (Variables|Default|GetTouchStartLocation) _output_get))) (Math|Float|Absolute(Float) (.y (- (Variables|Default|GetTouchStartLocation) _output_get))))
      (if (> (.x (- (Variables|Default|GetTouchStartLocation) _output_get)) 0.0)
        (CallFunction|MoveLeft)
        (else
          (CallFunction|MoveRight)))
      (elif (> (.y (- (Variables|Default|GetTouchStartLocation) _output_get)) 0.0)
        (CallFunction|MoveUp)
        (else
          (CallFunction|MoveDown))))))

(event Custom|SetControllType
  (params (ControllType :type EControllType%20Enum :default "NewEnumerator0"))
  ;[0 0 0] Set Controll Type
  (bind _output_get (Variables|Default|SetControllType ControllType))
  (switch Utilities|FlowControl|Switch|SwitchonEControllType _output_get
    (:NewEnumerator0
      (Variables|Default|SetbShowMouseCursor true)
      (Input|DisableInput 0))
    (:NewEnumerator1
      (Variables|Default|SetbShowMouseCursor false)
      (Input|EnableInput 0))))

(event Custom|SavePawnRef
  ;[0 0 0] Save Pawn Ref
  (bind _asbp_runner_player_pawn (Utilities|Casting|CastToBP_Runner_PlayerPawn (Pawn|GetControlledPawn)))
  (Variables|Default|SetBP_RunnerPlayerPawn _asbp_runner_player_pawn)
  (CallFunction|Binds))

(event Custom|MovePawnToCurrentLine
  ;[0 0 0] Move Pawn To Current Line
  (switch Utilities|FlowControl|Switch|SwitchonEControllType (Variables|Default|GetControllType)
    (:NewEnumerator1
      (Utilities|IsValid (Variables|Default|GetBP_MovingLevel)
        (:Is%20Valid
          _)
        (:Is%20Not%20Valid
          (bind _outactors (Actor|GetAllActorsOfClass "/Game/Source/Level/BP_MovingLevel_Straight_0.BP_MovingLevel_Straight_0_C"))
          (bind _output_get (Variables|Default|SetBP_MovingLevel (Utilities|Array|Get(acopy) _outactors)))))
      (bind _returnvalue (Class|MovingLevel|GetCurrentLine _output_get))
      (CallFunction|PawnMoveto _returnvalue))))

(event Custom|MoveDown
  ;[0 0 0] Moving Up
  (switch Utilities|FlowControl|Switch|SwitchonEControllType (Variables|Default|GetControllType)
    (:NewEnumerator1
      (Default|MovingDown (Variables|Default|GetBP_RunnerPlayerPawn)))))

(event Custom|MoveLeft
  ;[0 0 0] Line movement
  (switch Utilities|FlowControl|Switch|SwitchonEControllType (Variables|Default|GetControllType)
    (:NewEnumerator1
      (if (not (Variables|/Game/Source/BP_Runner_PlayerPawn.BP_Runner_PlayerPawn_C|GetInMovingYProcess (Variables|Default|GetBP_RunnerPlayerPawn)))
        (bind _returnvalue (Class|MovingLevel|MoveLeft (Variables|Default|GetBP_MovingLevel)))
        (CallFunction|PawnMoveto _returnvalue)))))

(event Custom|MoveRight
  ;[0 0 0] Line movement
  (switch Utilities|FlowControl|Switch|SwitchonEControllType (Variables|Default|GetControllType)
    (:NewEnumerator1
      (if (not (Variables|/Game/Source/BP_Runner_PlayerPawn.BP_Runner_PlayerPawn_C|GetInMovingYProcess (Variables|Default|GetBP_RunnerPlayerPawn)))
        (bind _returnvalue (Class|MovingLevel|MoveRight (Variables|Default|GetBP_MovingLevel)))
        (CallFunction|PawnMoveto _returnvalue)))))

(event EventBeginPlay)

(event Input|ActionEvents|InputActionMovingRight
  (params (Key :type Key%20Structure :default "None"))
  ;[0 0 0] Line movement
  (:Pressed
    (switch Utilities|FlowControl|Switch|SwitchonEControllType (Variables|Default|GetControllType)
      (:NewEnumerator1
        (if (not (Variables|/Game/Source/BP_Runner_PlayerPawn.BP_Runner_PlayerPawn_C|GetInMovingYProcess (Variables|Default|GetBP_RunnerPlayerPawn)))
          (bind _returnvalue (Class|MovingLevel|MoveRight (Variables|Default|GetBP_MovingLevel)))
          (CallFunction|PawnMoveto _returnvalue))))))

(event Input|ActionEvents|InputActionMovingLeft
  (params (Key :type Key%20Structure :default "None"))
  ;[0 0 0] Line movement
  (:Pressed
    (switch Utilities|FlowControl|Switch|SwitchonEControllType (Variables|Default|GetControllType)
      (:NewEnumerator1
        (if (not (Variables|/Game/Source/BP_Runner_PlayerPawn.BP_Runner_PlayerPawn_C|GetInMovingYProcess (Variables|Default|GetBP_RunnerPlayerPawn)))
          (bind _returnvalue (Class|MovingLevel|MoveLeft (Variables|Default|GetBP_MovingLevel)))
          (CallFunction|PawnMoveto _returnvalue))))))

(event Input|ActionEvents|InputActionMovingUp
  (params (Key :type Key%20Structure :default "None"))
  ;[0 0 0] Moving Up
  (:Pressed
    (switch Utilities|FlowControl|Switch|SwitchonEControllType (Variables|Default|GetControllType)
      (:NewEnumerator1
        (Default|MovingUp (Variables|Default|GetBP_RunnerPlayerPawn))))))

(event Input|ActionEvents|InputActionMovingDown
  (params (Key :type Key%20Structure :default "None"))
  ;[0 0 0] Moving Up
  (:Pressed
    (switch Utilities|FlowControl|Switch|SwitchonEControllType (Variables|Default|GetControllType)
      (:NewEnumerator1
        (Default|MovingDown (Variables|Default|GetBP_RunnerPlayerPawn))))))

(event Input|TouchEvents|InputTouch
  (params (Location :type Vector) (FingerIndex :type ETouchIndex%20Enum))
  ;[0 0 0] Mobile Controlls
  (:Pressed
    (Variables|Default|SetTouchStartLocation (Math|Vector2D|MakeVector2D (.x Location) (.y Location))))
  (:Released
    (Variables|Default|SetTouchEndLocation (Math|Vector2D|MakeVector2D (.x Location) (.y Location)))
    (CallFunction|CheckSwipe)))

(fn ConstructionScript)