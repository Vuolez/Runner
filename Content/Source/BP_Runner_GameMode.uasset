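; Game mode for a runner game that controls run start, continue and death around a moving level actor.
; BeginPlay caches the level and player controller, binds the pawn's death dispatcher and creates a save object.
; Run events start or stop the level and switch controller input modes, while a helper rolls back rows and returns the delay.
; Saving merges the run with the stored slot, keeping the best score and adding coins.
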(event Custom|StartRun
  (bind _bp_movinglevel (Variables|Default|GetBP_MovingLevel))
  (bind _bp_runner_player_controller (Variables|Default|GetBP%20Runner%20Player%20Controller))
  (Class|MovingLevel|Init _bp_movinglevel)
  (Class|MovingLevel|Start _bp_movinglevel)
  (Utilities|IsValid _bp_runner_player_controller
    (:Is%20Valid
      (Default|SetControllType _bp_runner_player_controller "NewEnumerator1")
      (Default|MovePawntoCurrentLine _bp_runner_player_controller))))

(event Custom|PlayerDeath
  (Class|MovingLevel|Stop (Variables|Default|GetBP_MovingLevel)))

(event Custom|Binds
  (bind _asbp_runner_player_pawn (Utilities|Casting|CastToBP_Runner_PlayerPawn (Game|Player|GetPlayerPawn 0)))
  (EventDispatchers|BindEventtoDeathDispatcher _asbp_runner_player_pawn (EventDispatchers|CreateEvent :!event Custom|PlayerDeath)))

(event Custom|ContinueRun
  (bind _bp_runner_player_controller (Variables|Default|GetBP%20Runner%20Player%20Controller))
  (Class|MovingLevel|Start (Variables|Default|GetBP_MovingLevel))
  (Utilities|IsValid _bp_runner_player_controller
    (:Is%20Valid
      (Default|SetControllType _bp_runner_player_controller "NewEnumerator1")
      (Default|MovePawntoCurrentLine _bp_runner_player_controller))))

(event EventBeginPlay
  (bind _outactors (Actor|GetAllActorsOfClass "/Game/Source/Level/BP_MovingLevel_Straight_0.BP_MovingLevel_Straight_0_C"))
  (Variables|Default|SetBP_MovingLevel (Utilities|Array|Get(acopy) _outactors))
  (bind _asbp_runner_player_controller (Utilities|Casting|CastToBP_Runner_PlayerController (Game|GetPlayerController 0)))
  (bind _output_get (Variables|Default|SetBP%20Runner%20Player%20Controller _asbp_runner_player_controller))
  (Default|SetControllType _output_get "NewEnumerator0")
  (CallFunction|Binds)
  (bind _returnvalue (SaveGame|CreateSaveGameObject "/Game/Source/BP_SaveGame.BP_SaveGame_C"))
  (Variables|Default|SetSaveGameInstance _returnvalue))

(fn ConstructionScript)

(fn RollBackRows
  (bind _bp_movinglevel (Variables|Default|GetBP_MovingLevel))
  (Class|MovingLevel|RollBackRow _bp_movinglevel 5)
  (bind _delay (Default|GetRollBackDelay _bp_movinglevel))
  (return _delay))

(fn LoadGame
  (bind _returnvalue (SaveGame|LoadGamefromSlot "MainPlayer"))
  (bind _asbp_save_game (Utilities|Casting|CastToBP_SaveGame _returnvalue))
  (return (Variables|/Game/Source/BP_SaveGame.BP_SaveGame_C|GetBestScore _asbp_save_game) (Variables|/Game/Source/BP_SaveGame.BP_SaveGame_C|GetCoins _asbp_save_game)))

(fn GetUpdatedSavingData
  (bind _savegameinstance (Variables|Default|GetSaveGameInstance))
  (bind (_bestscore _coints) (CallFunction|LoadGame))
  (Variables|/Game/Source/BP_SaveGame.BP_SaveGame_C|SetBestScore (Variables|Default|GetSaveGameInstance) (Math|Integer|Max(Integer) _bestscore (Math|Float|Truncate (Class|MovingLevel|GetScore (Variables|Default|GetBP_MovingLevel)))))
  (bind _returnvalue (Class|MovingLevel|GetCoins (Variables|Default|GetBP_MovingLevel)))
  (Variables|/Game/Source/BP_SaveGame.BP_SaveGame_C|SetCoins (Variables|Default|GetSaveGameInstance) (+ _returnvalue _coints))
  (return (Variables|/Game/Source/BP_SaveGame.BP_SaveGame_C|GetBestScore _savegameinstance) (Variables|/Game/Source/BP_SaveGame.BP_SaveGame_C|GetCoins _savegameinstance)))

(fn SaveGame
  (bind _savegameinstance (Variables|Default|GetSaveGameInstance))
  (bind _savegameinstance_2 (Variables|Default|GetSaveGameInstance))
  (bind (_bestscore _coins) (CallFunction|GetUpdatedSavingData))
  (Variables|/Game/Source/BP_SaveGame.BP_SaveGame_C|SetBestScore _savegameinstance _bestscore)
  (Variables|/Game/Source/BP_SaveGame.BP_SaveGame_C|SetCoins _savegameinstance _coins)
  (SaveGame|SaveGametoSlot _savegameinstance "MainPlayer")
  (return (Variables|/Game/Source/BP_SaveGame.BP_SaveGame_C|GetBestScore _savegameinstance_2) (Variables|/Game/Source/BP_SaveGame.BP_SaveGame_C|GetCoins _savegameinstance_2)))