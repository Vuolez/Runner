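; Player pawn for a runner game that handles timeline-driven movement, vertical camera shifts and a death notification.
; MovingUp and MovingDown feed MovingZ, which restarts a timeline on direction change to shift camera height by an offset while blending its start point toward the default.
; MoveTo lerps the actor to a target Y/Z at X zero, ignoring calls mid-move.
; Death fires a dispatcher, and an older camera-shift graph is left unconnected.
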(event Custom|MovingUp
  (CallFunction|MovingZ 1))

(event Custom|MovingZ
  (params (Direction :type Integer))
  (if (not (== Direction (Variables|Default|GetMovingZDirection)))
    (Variables|Default|SetMovingZDirection Direction)
    (Variables|Default|SetCameraStartLocation (Variables|/Script/Engine.SceneComponent|GetRelativeLocation (Variables|Default|GetCamera)))
    (bind _alpha (Timeline|UpDownTimeline PlayFromStart)
      (:Update
        (Transformation|SetRelativeLocation (Variables|Default|GetCamera) (Math|Vector|MakeVector (.x (Variables|Default|GetCameraStartLocation)) (.y (Variables|Default|GetCameraStartLocation)) (Math|Float|Lerp (.z (Variables|Default|GetCameraStartLocation)) (* (Variables|Default|GetUpDownOffset) (Math|Conversions|ToFloat(Integer) (Variables|Default|GetMovingZDirection))) _alpha)) false false)
        (Variables|Default|SetCameraStartLocation (Math|Vector|MakeVector (.x (Variables|Default|GetCameraStartLocation)) (.y (Variables|Default|GetCameraStartLocation)) (Math|Float|Lerp (.z (Variables|Default|GetCameraStartLocation)) (.z (Variables|Default|GetCameraDefaultLocation)) _alpha))))
      (:Finished
        (Variables|Default|SetMovingZDirection 0)))))

(event Custom|MovingDown
  (CallFunction|MovingZ -1))

(event Custom|MoveTo
  (params (TargetLocation :type Vector))
  (if (not (Variables|Default|GetInMovingYProcess))
    (Variables|Default|SetInMovingYProcess true)
    (Variables|Default|SetMoveToTarget%20Location (Math|Vector|MakeVector 0.0 (.y TargetLocation) (.z TargetLocation)))
    (Variables|Default|SetPawnDefaultLocation (Transformation|GetActorLocation))
    (bind _alpha (Timeline|MoveToTimeline PlayFromStart)
      (:Update
        (Transformation|SetActorLocation (Math|Vector|Lerp(Vector) (Variables|Default|GetPawnDefaultLocation) (Variables|Default|GetMoveToTarget%20Location) _alpha) false false))
      (:Finished
        (Variables|Default|SetInMovingYProcess false)))))

(event Custom|Death
  (Default|CallDeathDispatcher))

(event EventBeginPlay
  (Components|Timeline|SetPlayRate (Variables|Default|GetUpDownTimeline) (Variables|Default|GetUpDownRate))
  (Components|Timeline|SetPlayRate (Variables|Default|GetMoveToTimeline) (Variables|Default|GetMoveToRate))
  (Variables|Default|SetCameraDefaultLocation (Variables|/Script/Engine.SceneComponent|GetRelativeLocation (Variables|Default|GetCamera))))

(fn ConstructionScript)